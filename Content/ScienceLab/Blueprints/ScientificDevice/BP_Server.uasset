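; Server prop for the science lab that procedurally stacks static mesh modules in its construction script, with no runtime logic.
; The Random flag rerolls eleven module types and the vertical gaps between them, then clears itself to keep the layout.
; Each of six module types advances the Z offset by its height plus the gap.
; From the sixth module on, a type-specific height limit ends the stack once a module won't fit.
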(fn `UserConstructionScript`
  (bind _returnvalue (`KismetMathLibrary.RandomInteger` 6))
  (bind _returnvalue_2 (`KismetMathLibrary.RandomFloatInRange` -1.0 5.0))
  (bind _returnvalue_3 (`KismetMathLibrary.Conv_VectorToTransform` (`self.Location 4`)))
  (bind _returnvalue_4 (`KismetMathLibrary.Conv_VectorToTransform` (`self.Location 5`)))
  (bind _returnvalue_5 (`KismetMathLibrary.Conv_VectorToTransform` (`self.Location 6`)))
  (bind _returnvalue_6 (`KismetMathLibrary.Conv_VectorToTransform` (`self.Location 7`)))
  (bind _returnvalue_7 (`KismetMathLibrary.Conv_VectorToTransform` (`self.Location 8`)))
  (bind _returnvalue_8 (`KismetMathLibrary.Conv_VectorToTransform` (`self.Location 9`)))
  (bind _returnvalue_9 (`KismetMathLibrary.Conv_VectorToTransform` (`self.Location 10`)))
  (bind _z (.z (`self.Location 10`)))
  (bind _z_2 (.z (`self.Location 6`)))
  (bind _z_3 (.z (`self.Location 7`)))
  (bind _z_4 (.z (`self.Location 8`)))
  (bind _z_5 (.z (`self.Location 9`)))
  (bind _z_6 (.z (`self.Location 5`)))
  (bind _returnvalue_10 (`KismetMathLibrary.Conv_VectorToTransform` (`self.Location 1`)))
  (bind _returnvalue_11 (`KismetMathLibrary.Conv_VectorToTransform` (`self.Location 2`)))
  (bind _returnvalue_12 (`KismetMathLibrary.Conv_VectorToTransform` (`self.Location 3`)))
  (bind _returnvalue_13 (`KismetMathLibrary.MakeVector` 0.0 0.0 (+ (`self.Random Int 01`) (.z (0.0 0.0 0.0)))))
  (bind _returnvalue_14 (`KismetMathLibrary.MakeVector` 0.0 0.0 (+ (`self.Random Int 10`) (.z (`self.Location 9`)))))
  (bind _returnvalue_15 (`KismetMathLibrary.MakeVector` 0.0 0.0 (+ (`self.Random Int 02`) (.z (`self.Location 1`)))))
  (bind _returnvalue_16 (`KismetMathLibrary.MakeVector` 0.0 0.0 (+ (`self.Random Int 03`) (.z (`self.Location 2`)))))
  (bind _returnvalue_17 (`KismetMathLibrary.MakeVector` 0.0 0.0 (+ (`self.Random Int 04`) (.z (`self.Location 3`)))))
  (bind _returnvalue_18 (`KismetMathLibrary.MakeVector` 0.0 0.0 (+ (`self.Random Int 05`) (.z (`self.Location 4`)))))
  (bind _returnvalue_19 (`KismetMathLibrary.MakeVector` 0.0 0.0 (+ (`self.Random Int 06`) (.z (`self.Location 5`)))))
  (bind _returnvalue_20 (`KismetMathLibrary.MakeVector` 0.0 0.0 (+ (`self.Random Int 07`) (.z (`self.Location 6`)))))
  (bind _returnvalue_21 (`KismetMathLibrary.MakeVector` 0.0 0.0 (+ (`self.Random Int 08`) (.z (`self.Location 7`)))))
  (bind _returnvalue_22 (`KismetMathLibrary.MakeVector` 0.0 0.0 (+ (`self.Random Int 09`) (.z (`self.Location 8`)))))
  (if (`self.Random`)
    (set `self.Module 1 ` _returnvalue)
    (set `self.Module 2` _returnvalue)
    (set `self.Module 3` _returnvalue)
    (set `self.Module 4` _returnvalue)
    (set `self.Module 5` _returnvalue)
    (set `self.Module 6` _returnvalue)
    (set `self.Module 7` _returnvalue)
    (set `self.Module 8` _returnvalue)
    (set `self.Module 9` _returnvalue)
    (set `self.Module 10` _returnvalue)
    (set `self.Module 11` _returnvalue)
    (set `self.Random Int 01` _returnvalue_2)
    (set `self.Random Int 02` _returnvalue_2)
    (set `self.Random Int 03` _returnvalue_2)
    (set `self.Random Int 04` _returnvalue_2)
    (set `self.Random Int 05` _returnvalue_2)
    (set `self.Random Int 06` _returnvalue_2)
    (set `self.Random Int 07` _returnvalue_2)
    (set `self.Random Int 08` _returnvalue_2)
    (set `self.Random Int 09` _returnvalue_2)
    (set `self.Random Int 10` _returnvalue_2)
    (set `self.Random` false))
  ;[1 1 1] MODULE 01
  (switch `int` (`self.Module 1 `)
    (:`Default`
      (`AddComponent|NODE_AddStaticMeshComponent-0` :!label _label)
      (set `self.Location 1` (+ _returnvalue_13 (0.0 0.0 20.0))))
    (:`0`
      (goto _label))
    (:`1`
      (`AddComponent|NODE_AddStaticMeshComponent-3`)
      (set `self.Location 1` (+ _returnvalue_13 (0.0 0.0 24.0))))
    (:`2`
      (`AddComponent|NODE_AddStaticMeshComponent-4`)
      (set `self.Location 1` (+ _returnvalue_13 (0.0 0.0 36.0))))
    (:`3`
      (`AddComponent|NODE_AddStaticMeshComponent-5`)
      (set `self.Location 1` (+ _returnvalue_13 (0.0 0.0 30.0))))
    (:`4`
      (`AddComponent|NODE_AddStaticMeshComponent-6`)
      (set `self.Location 1` (+ _returnvalue_13 (0.0 0.0 44.0))))
    (:`5`
      (`AddComponent|NODE_AddStaticMeshComponent-7`)
      (set `self.Location 1` (+ _returnvalue_13 (0.0 0.0 36.0)))))
  ;[1 1 1] MODULE 02
  (switch `int` (`self.Module 2`)
    (:`Default`
      (`AddComponent|NODE_AddStaticMeshComponent-9` :`RelativeTransform` _returnvalue_10 :!label _label_2)
      (set `self.Location 2` (+ _returnvalue_15 (0.0 0.0 20.0))))
    (:`0`
      (goto _label_2))
    (:`1`
      (`AddComponent|NODE_AddStaticMeshComponent-10` :`RelativeTransform` _returnvalue_10)
      (set `self.Location 2` (+ _returnvalue_15 (0.0 0.0 24.0))))
    (:`2`
      (`AddComponent|NODE_AddStaticMeshComponent-11` :`RelativeTransform` _returnvalue_10)
      (set `self.Location 2` (+ _returnvalue_15 (0.0 0.0 36.0))))
    (:`3`
      (`AddComponent|NODE_AddStaticMeshComponent-12` :`RelativeTransform` _returnvalue_10)
      (set `self.Location 2` (+ _returnvalue_15 (0.0 0.0 30.0))))
    (:`4`
      (`AddComponent|NODE_AddStaticMeshComponent-13` :`RelativeTransform` _returnvalue_10)
      (set `self.Location 2` (+ _returnvalue_15 (0.0 0.0 44.0))))
    (:`5`
      (`AddComponent|NODE_AddStaticMeshComponent-14` :`RelativeTransform` _returnvalue_10)
      (set `self.Location 2` (+ _returnvalue_15 (0.0 0.0 36.0)))))
  ;[1 1 1] MODULE 03
  (switch `int` (`self.Module 3`)
    (:`Default`
      (`AddComponent|NODE_AddStaticMeshComponent-22` :`RelativeTransform` _returnvalue_11 :!label _label_3)
      (set `self.Location 3` (+ _returnvalue_16 (0.0 0.0 20.0))))
    (:`0`
      (goto _label_3))
    (:`1`
      (`AddComponent|NODE_AddStaticMeshComponent-23` :`RelativeTransform` _returnvalue_11)
      (set `self.Location 3` (+ _returnvalue_16 (0.0 0.0 24.0))))
    (:`2`
      (`AddComponent|NODE_AddStaticMeshComponent-24` :`RelativeTransform` _returnvalue_11)
      (set `self.Location 3` (+ _returnvalue_16 (0.0 0.0 36.0))))
    (:`3`
      (`AddComponent|NODE_AddStaticMeshComponent-25` :`RelativeTransform` _returnvalue_11)
      (set `self.Location 3` (+ _returnvalue_16 (0.0 0.0 30.0))))
    (:`4`
      (`AddComponent|NODE_AddStaticMeshComponent-26` :`RelativeTransform` _returnvalue_11)
      (set `self.Location 3` (+ _returnvalue_16 (0.0 0.0 44.0))))
    (:`5`
      (`AddComponent|NODE_AddStaticMeshComponent-27` :`RelativeTransform` _returnvalue_11)
      (set `self.Location 3` (+ _returnvalue_16 (0.0 0.0 36.0)))))
  ;[1 1 1] MODULE 04
  (switch `int` (`self.Module 4`)
    (:`Default`
      (`AddComponent|NODE_AddStaticMeshComponent-28` :`RelativeTransform` _returnvalue_12 :!label _label_4)
      (set `self.Location 4` (+ _returnvalue_17 (0.0 0.0 20.0))))
    (:`0`
      (goto _label_4))
    (:`1`
      (`AddComponent|NODE_AddStaticMeshComponent-29` :`RelativeTransform` _returnvalue_12)
      (set `self.Location 4` (+ _returnvalue_17 (0.0 0.0 24.0))))
    (:`2`
      (`AddComponent|NODE_AddStaticMeshComponent-30` :`RelativeTransform` _returnvalue_12)
      (set `self.Location 4` (+ _returnvalue_17 (0.0 0.0 36.0))))
    (:`3`
      (`AddComponent|NODE_AddStaticMeshComponent-31` :`RelativeTransform` _returnvalue_12)
      (set `self.Location 4` (+ _returnvalue_17 (0.0 0.0 30.0))))
    (:`4`
      (`AddComponent|NODE_AddStaticMeshComponent-32` :`RelativeTransform` _returnvalue_12)
      (set `self.Location 4` (+ _returnvalue_17 (0.0 0.0 44.0))))
    (:`5`
      (`AddComponent|NODE_AddStaticMeshComponent-33` :`RelativeTransform` _returnvalue_12)
      (set `self.Location 4` (+ _returnvalue_17 (0.0 0.0 36.0)))))
  ;[1 1 1] MODULE 05
  (switch `int` (`self.Module 5`)
    (:`Default`
      (`AddComponent|NODE_AddStaticMeshComponent-34` :`RelativeTransform` _returnvalue_3 :!label _label_5)
      (set `self.Location 5` (+ _returnvalue_18 (0.0 0.0 20.0))))
    (:`0`
      (goto _label_5))
    (:`1`
      (`AddComponent|NODE_AddStaticMeshComponent-35` :`RelativeTransform` _returnvalue_3)
      (set `self.Location 5` (+ _returnvalue_18 (0.0 0.0 24.0))))
    (:`2`
      (`AddComponent|NODE_AddStaticMeshComponent-36` :`RelativeTransform` _returnvalue_3)
      (set `self.Location 5` (+ _returnvalue_18 (0.0 0.0 36.0))))
    (:`3`
      (`AddComponent|NODE_AddStaticMeshComponent-37` :`RelativeTransform` _returnvalue_3)
      (set `self.Location 5` (+ _returnvalue_18 (0.0 0.0 30.0))))
    (:`4`
      (`AddComponent|NODE_AddStaticMeshComponent-38` :`RelativeTransform` _returnvalue_3)
      (set `self.Location 5` (+ _returnvalue_18 (0.0 0.0 44.0))))
    (:`5`
      (`AddComponent|NODE_AddStaticMeshComponent-39` :`RelativeTransform` _returnvalue_3)
      (set `self.Location 5` (+ _returnvalue_18 (0.0 0.0 36.0)))))
  ;[1 1 1] MODULE 06
  (switch `int` (`self.Module 6`)
    (:`Default`
      (`/Engine/EditorBlueprintResources/StandardMacros.CompareFloat` _z_6 198.0 :!label _label_6
        (:`<`
          (`AddComponent|NODE_AddStaticMeshComponent-40` :`RelativeTransform` _returnvalue_4)
          (set `self.Location 6` (+ _returnvalue_19 (0.0 0.0 20.0))))))
    (:`0`
      (goto _label_6))
    (:`1`
      (`/Engine/EditorBlueprintResources/StandardMacros.CompareFloat` _z_6 194.0
        (:`<`
          (`AddComponent|NODE_AddStaticMeshComponent-41` :`RelativeTransform` _returnvalue_4)
          (set `self.Location 6` (+ _returnvalue_19 (0.0 0.0 24.0))))))
    (:`2`
      (`/Engine/EditorBlueprintResources/StandardMacros.CompareFloat` _z_6 184.0
        (:`<`
          (`AddComponent|NODE_AddStaticMeshComponent-42` :`RelativeTransform` _returnvalue_4)
          (set `self.Location 6` (+ _returnvalue_19 (0.0 0.0 36.0))))))
    (:`3`
      (`/Engine/EditorBlueprintResources/StandardMacros.CompareFloat` _z_6 188.0
        (:`<`
          (`AddComponent|NODE_AddStaticMeshComponent-43` :`RelativeTransform` _returnvalue_4)
          (set `self.Location 6` (+ _returnvalue_19 (0.0 0.0 30.0))))))
    (:`4`
      (`/Engine/EditorBlueprintResources/StandardMacros.CompareFloat` _z_6 176.0
        (:`<`
          (`AddComponent|NODE_AddStaticMeshComponent-44` :`RelativeTransform` _returnvalue_4)
          (set `self.Location 6` (+ _returnvalue_19 (0.0 0.0 44.0))))))
    (:`5`
      (`/Engine/EditorBlueprintResources/StandardMacros.CompareFloat` _z_6 184.0
        (:`<`
          (`AddComponent|NODE_AddStaticMeshComponent-45` :`RelativeTransform` _returnvalue_4)
          (set `self.Location 6` (+ _returnvalue_19 (0.0 0.0 36.0)))))))
  ;[1 1 1] MODULE 07
  (switch `int` (`self.Module 7`)
    (:`Default`
      (`/Engine/EditorBlueprintResources/StandardMacros.CompareFloat` _z_2 198.0 :!label _label_7
        (:`<`
          (`AddComponent|NODE_AddStaticMeshComponent-52` :`RelativeTransform` _returnvalue_5)
          (set `self.Location 7` (+ _returnvalue_20 (0.0 0.0 20.0))))))
    (:`0`
      (goto _label_7))
    (:`1`
      (`/Engine/EditorBlueprintResources/StandardMacros.CompareFloat` _z_2 194.0
        (:`<`
          (`AddComponent|NODE_AddStaticMeshComponent-53` :`RelativeTransform` _returnvalue_5)
          (set `self.Location 7` (+ _returnvalue_20 (0.0 0.0 24.0))))))
    (:`2`
      (`/Engine/EditorBlueprintResources/StandardMacros.CompareFloat` _z_2 184.0
        (:`<`
          (`AddComponent|NODE_AddStaticMeshComponent-54` :`RelativeTransform` _returnvalue_5)
          (set `self.Location 7` (+ _returnvalue_20 (0.0 0.0 36.0))))))
    (:`3`
      (`/Engine/EditorBlueprintResources/StandardMacros.CompareFloat` _z_2 188.0
        (:`<`
          (`AddComponent|NODE_AddStaticMeshComponent-55` :`RelativeTransform` _returnvalue_5)
          (set `self.Location 7` (+ _returnvalue_20 (0.0 0.0 30.0))))))
    (:`4`
      (`/Engine/EditorBlueprintResources/StandardMacros.CompareFloat` _z_2 176.0
        (:`<`
          (`AddComponent|NODE_AddStaticMeshComponent-56` :`RelativeTransform` _returnvalue_5)
          (set `self.Location 7` (+ _returnvalue_20 (0.0 0.0 44.0))))))
    (:`5`
      (`/Engine/EditorBlueprintResources/StandardMacros.CompareFloat` _z_2 184.0
        (:`<`
          (`AddComponent|NODE_AddStaticMeshComponent-57` :`RelativeTransform` _returnvalue_5)
          (set `self.Location 7` (+ _returnvalue_20 (0.0 0.0 36.0)))))))
  ;[1 1 1] MODULE 08
  (switch `int` (`self.Module 8`)
    (:`Default`
      (`/Engine/EditorBlueprintResources/StandardMacros.CompareFloat` _z_3 198.0 :!label _label_8
        (:`<`
          (`AddComponent|NODE_AddStaticMeshComponent-58` :`RelativeTransform` _returnvalue_6)
          (set `self.Location 8` (+ _returnvalue_21 (0.0 0.0 20.0))))))
    (:`0`
      (goto _label_8))
    (:`1`
      (`/Engine/EditorBlueprintResources/StandardMacros.CompareFloat` _z_3 194.0
        (:`<`
          (`AddComponent|NODE_AddStaticMeshComponent-59` :`RelativeTransform` _returnvalue_6)
          (set `self.Location 8` (+ _returnvalue_21 (0.0 0.0 24.0))))))
    (:`2`
      (`/Engine/EditorBlueprintResources/StandardMacros.CompareFloat` _z_3 184.0
        (:`<`
          (`AddComponent|NODE_AddStaticMeshComponent-60` :`RelativeTransform` _returnvalue_6)
          (set `self.Location 8` (+ _returnvalue_21 (0.0 0.0 36.0))))))
    (:`3`
      (`/Engine/EditorBlueprintResources/StandardMacros.CompareFloat` _z_3 188.0
        (:`<`
          (`AddComponent|NODE_AddStaticMeshComponent-61` :`RelativeTransform` _returnvalue_6)
          (set `self.Location 8` (+ _returnvalue_21 (0.0 0.0 30.0))))))
    (:`4`
      (`/Engine/EditorBlueprintResources/StandardMacros.CompareFloat` _z_3 176.0
        (:`<`
          (`AddComponent|NODE_AddStaticMeshComponent-62` :`RelativeTransform` _returnvalue_6)
          (set `self.Location 8` (+ _returnvalue_21 (0.0 0.0 44.0))))))
    (:`5`
      (`/Engine/EditorBlueprintResources/StandardMacros.CompareFloat` _z_3 184.0
        (:`<`
          (`AddComponent|NODE_AddStaticMeshComponent-63` :`RelativeTransform` _returnvalue_6)
          (set `self.Location 8` (+ _returnvalue_21 (0.0 0.0 36.0)))))))
  ;[1 1 1] MODULE 09
  (switch `int` (`self.Module 9`)
    (:`Default`
      (`/Engine/EditorBlueprintResources/StandardMacros.CompareFloat` _z_4 198.0 :!label _label_9
        (:`<`
          (`AddComponent|NODE_AddStaticMeshComponent-64` :`RelativeTransform` _returnvalue_7)
          (set `self.Location 9` (+ _returnvalue_22 (0.0 0.0 20.0))))))
    (:`0`
      (goto _label_9))
    (:`1`
      (`/Engine/EditorBlueprintResources/StandardMacros.CompareFloat` _z_4 194.0
        (:`<`
          (`AddComponent|NODE_AddStaticMeshComponent-65` :`RelativeTransform` _returnvalue_7)
          (set `self.Location 9` (+ _returnvalue_22 (0.0 0.0 24.0))))))
    (:`2`
      (`/Engine/EditorBlueprintResources/StandardMacros.CompareFloat` _z_4 184.0
        (:`<`
          (`AddComponent|NODE_AddStaticMeshComponent-66` :`RelativeTransform` _returnvalue_7)
          (set `self.Location 9` (+ _returnvalue_22 (0.0 0.0 36.0))))))
    (:`3`
      (`/Engine/EditorBlueprintResources/StandardMacros.CompareFloat` _z_4 188.0
        (:`<`
          (`AddComponent|NODE_AddStaticMeshComponent-67` :`RelativeTransform` _returnvalue_7)
          (set `self.Location 9` (+ _returnvalue_22 (0.0 0.0 30.0))))))
    (:`4`
      (`/Engine/EditorBlueprintResources/StandardMacros.CompareFloat` _z_4 176.0
        (:`<`
          (`AddComponent|NODE_AddStaticMeshComponent-68` :`RelativeTransform` _returnvalue_7)
          (set `self.Location 9` (+ _returnvalue_22 (0.0 0.0 44.0))))))
    (:`5`
      (`/Engine/EditorBlueprintResources/StandardMacros.CompareFloat` _z_4 184.0
        (:`<`
          (`AddComponent|NODE_AddStaticMeshComponent-69` :`RelativeTransform` _returnvalue_7)
          (set `self.Location 9` (+ _returnvalue_22 (0.0 0.0 36.0)))))))
  ;[1 1 1] MODULE 10
  (switch `int` (`self.Module 10`)
    (:`Default`
      (`/Engine/EditorBlueprintResources/StandardMacros.CompareFloat` _z_5 198.0 :!label _label_10
        (:`<`
          (`AddComponent|NODE_AddStaticMeshComponent-70` :`RelativeTransform` _returnvalue_8)
          (set `self.Location 10` (+ _returnvalue_14 (0.0 0.0 20.0))))))
    (:`0`
      (goto _label_10))
    (:`1`
      (`/Engine/EditorBlueprintResources/StandardMacros.CompareFloat` _z_5 194.0
        (:`<`
          (`AddComponent|NODE_AddStaticMeshComponent-71` :`RelativeTransform` _returnvalue_8)
          (set `self.Location 10` (+ _returnvalue_14 (0.0 0.0 24.0))))))
    (:`2`
      (`/Engine/EditorBlueprintResources/StandardMacros.CompareFloat` _z_5 184.0
        (:`<`
          (`AddComponent|NODE_AddStaticMeshComponent-72` :`RelativeTransform` _returnvalue_8)
          (set `self.Location 10` (+ _returnvalue_14 (0.0 0.0 36.0))))))
    (:`3`
      (`/Engine/EditorBlueprintResources/StandardMacros.CompareFloat` _z_5 188.0
        (:`<`
          (`AddComponent|NODE_AddStaticMeshComponent-73` :`RelativeTransform` _returnvalue_8)
          (set `self.Location 10` (+ _returnvalue_14 (0.0 0.0 30.0))))))
    (:`4`
      (`/Engine/EditorBlueprintResources/StandardMacros.CompareFloat` _z_5 176.0
        (:`<`
          (`AddComponent|NODE_AddStaticMeshComponent-74` :`RelativeTransform` _returnvalue_8)
          (set `self.Location 10` (+ _returnvalue_14 (0.0 0.0 44.0))))))
    (:`5`
      (`/Engine/EditorBlueprintResources/StandardMacros.CompareFloat` _z_5 184.0
        (:`<`
          (`AddComponent|NODE_AddStaticMeshComponent-75` :`RelativeTransform` _returnvalue_8)
          (set `self.Location 10` (+ _returnvalue_14 (0.0 0.0 36.0)))))))
  ;[1 1 1] MODULE 11
  (switch `int` (`self.Module 11`)
    (:`Default`
      (`/Engine/EditorBlueprintResources/StandardMacros.CompareFloat` _z 198.0 :!label _label_11
        (:`<`
          (`AddComponent|NODE_AddStaticMeshComponent-76` :`RelativeTransform` _returnvalue_9))))
    (:`0`
      (goto _label_11))
    (:`1`
      (`/Engine/EditorBlueprintResources/StandardMacros.CompareFloat` _z 194.0
        (:`<`
          (`AddComponent|NODE_AddStaticMeshComponent-77` :`RelativeTransform` _returnvalue_9))))
    (:`2`
      (`/Engine/EditorBlueprintResources/StandardMacros.CompareFloat` _z 184.0
        (:`<`
          (`AddComponent|NODE_AddStaticMeshComponent-78` :`RelativeTransform` _returnvalue_9))))
    (:`3`
      (`/Engine/EditorBlueprintResources/StandardMacros.CompareFloat` _z 188.0
        (:`<`
          (`AddComponent|NODE_AddStaticMeshComponent-79` :`RelativeTransform` _returnvalue_9))))
    (:`4`
      (`/Engine/EditorBlueprintResources/StandardMacros.CompareFloat` _z 176.0
        (:`<`
          (`AddComponent|NODE_AddStaticMeshComponent-80` :`RelativeTransform` _returnvalue_9))))
    (:`5`
      (`/Engine/EditorBlueprintResources/StandardMacros.CompareFloat` _z 184.0
        (:`<`
          (`AddComponent|NODE_AddStaticMeshComponent-81` :`RelativeTransform` _returnvalue_9))))))